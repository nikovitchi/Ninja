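; BP_NinjaAA is an actor that deals one hit of damage on contact and then destroys itself.
; Its BoxCollision begin-overlap checks the other component for the "IsDamagable" tag and passes that component's owning actor to DamageIt, which applies DamageCaused and removes this actor.
; The construction script only prints a debug string when the instigator equals Turret.
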(event `self.DamageIt`
  (params (ToWho :type "Actor Object Reference"))
  ;[1 1 1] Damage Function
  (`GameplayStatics.ApplyDamage` ToWho (`self.DamageCaused`))
  (`self.K2_DestroyActor`))

(event `self.BoxCollision.OnComponentBeginOverlap`
  (params (OverlappedComponent :type "PrimitiveComponent Object Reference") (OtherActor :type "Actor Object Reference") (OtherComp :type "PrimitiveComponent Object Reference") (OtherBodyIndex :type Integer) (bFromSweep :type Boolean) (SweepResult :type "HitResult Structure (by ref)"))
  (if (`ActorComponent.ComponentHasTag` OtherComp "IsDamagable")
    (`self.DamageIt` OtherActor)))

(fn `UserConstructionScript`
  (if (== (`self.GetInstigator`) "/Game/DaGame/Turret.Turret")
    (`KismetSystemLibrary.PrintString` "ih")))